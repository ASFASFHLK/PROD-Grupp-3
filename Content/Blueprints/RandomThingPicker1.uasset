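; RandomThingPicker1 is a Blueprint that shows and plays one of three sound variants: normal, pitch-changed or volume-changed.
; On BeginPlay it reads PlayNumber from the SoundChange_GI game instance and writes the matching variant name to a text render.
; The same number then selects which 2D sound plays: the music box loop, NewPitch or NewVolume.
; The selection is not randomized here, despite the asset name.
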(event EventBeginPlay
  (bind _assound_change_gi (Utilities|Casting|CastToSoundChange_GI (Game|GetGameInstance)))
  (Variables|Default|SetPlay%20number (Variables|/Game/Blueprints/SoundChange_GI.SoundChange_GI_C|GetPlay%20Number _assound_change_gi))
  (switch int (Variables|Default|GetPlay%20number)
    (:0
      (Variables|Default|SetSoundChange "Normal"))
    (:1
      (Variables|Default|SetSoundChange "Pitch"))
    (:2
      (Variables|Default|SetSoundChange "Volume")))
  (Rendering|Components|TextRender|SetText (Variables|Default|GetTextRender) (Variables|Default|GetSoundChange))
  (switch int (Variables|Default|GetPlay%20number)
    (:Default
      (Audio|PlaySound2D "/Game/Sounds/752555__twotrickpony__dance-of-the-melancholy-marionettes-dark-music-box-melody-loop.752555__twotrickpony__dance-of-the-melancholy-marionettes-dark-music-box-melody-loop" 1.0 1.0 0.0 0 0 :!label _label))
    (:0
      (goto _label))
    (:1
      (Audio|PlaySound2D "/Game/Sounds/NewPitch.NewPitch" 1.0 1.0 0.0 0 0))
    (:2
      (Audio|PlaySound2D "/Game/Sounds/NewVolume.NewVolume" 1.0 1.0 0.0 0 0))))

(fn ConstructionScript)