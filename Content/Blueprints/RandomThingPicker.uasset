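; Actor that randomly picks Volume or Pitch as the current sound change when play begins.
; It shows the chosen name on a TextRender and writes the number to PlayNumber in SoundChange_GI, making it available through the game instance.
; It then plays the matching 2D sound, NewVolume or NewPitch.
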(event EventBeginPlay
  (Variables|Default|SetPlay%20number 0)
  (Variables|Default|SetPlay%20number (Math|Random|RandomIntegerinRange 0 1))
  (switch int (Variables|Default|GetPlay%20number)
    (:0
      (Variables|Default|SetSoundChange "Volume"))
    (:1
      (Variables|Default|SetSoundChange "Pitch")))
  (Rendering|Components|TextRender|SetText (Variables|Default|GetTextRender) (Variables|Default|GetSoundChange))
  (bind _assound_change_gi (Utilities|Casting|CastToSoundChange_GI (Game|GetGameInstance)))
  (Variables|/Game/Blueprints/SoundChange_GI.SoundChange_GI_C|SetPlay%20Number _assound_change_gi (Variables|Default|GetPlay%20number))
  (switch int (Variables|Default|GetPlay%20number)
    (:0
      (Audio|PlaySound2D "/Game/Sounds/NewVolume.NewVolume" 1.0 1.0 0.0 0 0))
    (:1
      (Audio|PlaySound2D "/Game/Sounds/NewPitch.NewPitch" 1.0 1.0 0.0 0 0))))

(fn ConstructionScript)