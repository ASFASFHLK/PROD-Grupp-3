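; Main menu pawn that gives keyboard control over a two-option Start/Quit menu.
; Releasing W or S toggles the selection between Start and Quit and plays a sound for the newly selected option.
; Releasing Space casts the game mode to GMBP_MainMenu and calls its MainMenu's start or quit click event to match the selection.
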(event Collision|EventActorBeginOverlap
  (params (OtherActor :type Actor%20Object%20Reference)))

(event EventTick
  (params (DeltaSeconds :type Float%20%28single-precision%29)))

(event Input|KeyboardEvents|SpaceBar
  (params (Key :type Key%20Structure :default "None"))
  (:Released
    (bind _asgmbp_main_menu (Utilities|Casting|CastToGMBP_MainMenu (Game|GetGameMode)))
    (if (Variables|Default|GetSelectedStart)
      (Default|StartGameonClickedEvent (Variables|/Game/Blueprints/GMBP_MainMenu.GMBP_MainMenu_C|GetMain%20Menu _asgmbp_main_menu))
      (else
        (Default|QuitGameonClickedEvent (Variables|/Game/Blueprints/GMBP_MainMenu.GMBP_MainMenu_C|GetMain%20Menu _asgmbp_main_menu))))))

(event Input|KeyboardEvents|S
  (params (Key :type Key%20Structure :default "None"))
  (:Released
    (Variables|Default|SetSelectedStart (not (Variables|Default|GetSelectedStart)))
    (if (Variables|Default|GetSelectedStart)
      (Audio|PlaySound2D "/Game/Sounds/MainMenu/StartGame.StartGame" 1.0 1.0 0.0 0 0)
      (else
        (Audio|PlaySound2D "/Game/Sounds/MainMenu/Quit.Quit" 1.0 1.0 0.0 0 0)))))

(event Input|KeyboardEvents|W
  (params (Key :type Key%20Structure :default "None"))
  (:Released
    (Variables|Default|SetSelectedStart (not (Variables|Default|GetSelectedStart)))
    (if (Variables|Default|GetSelectedStart)
      (Audio|PlaySound2D "/Game/Sounds/MainMenu/StartGame.StartGame" 1.0 1.0 0.0 0 0)
      (else
        (Audio|PlaySound2D "/Game/Sounds/MainMenu/Quit.Quit" 1.0 1.0 0.0 0 0)))))

(fn ConstructionScript)