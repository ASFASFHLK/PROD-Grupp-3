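; SoundPlayer is an actor that serves as a spooky sound source and ghost spawn point when picked.
; On Picked, it plays whispers, spawns a BP_GhostLocation at its transform, and loads a random spooky sound into its Audio component without playing it.
; It hands the audio component, whispers and spawned actor (as DestroyMe) to BP_FirstPersonCharacter.
; ResetValues restores and plays the default sound.
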(event Custom|Picked
  (bind _self self)
  (bind _returnvalue (Audio|SpawnSoundatLocation (Variables|Default|GetWhispers) (Transformation|GetActorLocation) "0, 0, 0" 1.0 1.0 0.0 0 0))
  (bind _returnvalue_2 (Game|SpawnActorfromClass "/Game/FirstPerson/Blueprints/BP_GhostLocation.BP_GhostLocation_C" (Transformation|GetActorTransform _self) "Undefined" "MultiplyWithRoot" _self 0))
  (bind _output_get (Variables|Default|SetDestroyable _returnvalue_2))
  (Audio|Components|Audio|SetSound (Variables|Default|GetAudio) (.OutItem (Utilities|Array|Random (Variables|Default|GetSpookySounds))))
  (bind _asbp_first_person_character (Utilities|Casting|CastToBP_FirstPersonCharacter (Game|GetPlayerCharacter 0)))
  (Variables|/Game/FirstPerson/Blueprints/BP_FirstPersonCharacter.BP_FirstPersonCharacter_C|Setspooky%20sound _asbp_first_person_character (Variables|Default|GetAudio))
  (bind _asbp_first_person_character_2 (Utilities|Casting|CastToBP_FirstPersonCharacter (Game|GetPlayerCharacter 0)))
  (Variables|/Game/FirstPerson/Blueprints/BP_FirstPersonCharacter.BP_FirstPersonCharacter_C|SetWhispers _asbp_first_person_character_2 _returnvalue)
  (Variables|/Game/FirstPerson/Blueprints/BP_FirstPersonCharacter.BP_FirstPersonCharacter_C|SetDestroy%20me _asbp_first_person_character_2 _output_get))

(event Custom|ResetValues
  (Audio|Components|Audio|SetSound (Variables|Default|GetAudio) (Variables|Default|GetDefault_sound))
  (Audio|Components|Audio|Play (Variables|Default|GetAudio) 0.0))

(fn ConstructionScript)