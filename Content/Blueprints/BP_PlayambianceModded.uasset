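; BP_PlayambianceModded is a trigger-volume actor that plays a non-spatial ambience cue for the first-person character.
; It spawns AmbiantSoundCue as a 2D sound on BeginPlay and again whenever the character enters its Box, storing the result in AmbianceSound.
; Leaving the Box stops only that stored sound.
; Each spawn overwrites the reference without stopping the previous sound, so the BeginPlay instance is orphaned on first entry.
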(event OnComponentBeginOverlap(Box)
  (params (OverlappedComponent :type Primitive%20Component%20Object%20Reference) (OtherActor :type Actor%20Object%20Reference) (OtherComp :type Primitive%20Component%20Object%20Reference) (OtherBodyIndex :type Integer) (bFromSweep :type Boolean) (SweepResult :type Hit%20Result%20Structure%20%28by%20ref%29))
  (Utilities|Casting|CastToBP_FirstPersonCharacter OtherActor)
  (bind _returnvalue (Audio|SpawnSound2D (Variables|Default|GetAmbiantSoundCue) 1.0 1.0 0.0 0))
  (Variables|Default|SetAmbianceSound _returnvalue))

(event OnComponentEndOverlap(Box)
  (params (OverlappedComponent :type Primitive%20Component%20Object%20Reference) (OtherActor :type Actor%20Object%20Reference) (OtherComp :type Primitive%20Component%20Object%20Reference) (OtherBodyIndex :type Integer))
  (Utilities|Casting|CastToBP_FirstPersonCharacter OtherActor)
  (Audio|Components|Audio|Stop (Variables|Default|GetAmbianceSound)))

(event EventBeginPlay
  (bind _returnvalue (Audio|SpawnSound2D (Variables|Default|GetAmbiantSoundCue) 1.0 1.0 0.0 0))
  (Variables|Default|SetAmbianceSound _returnvalue))

(fn ConstructionScript)